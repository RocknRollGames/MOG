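; MOG card table actor that defines where cards lie for the stock, two players' suit piles and neutral suit piles.
; Placement functions ask MOGGameModeBase for the pile's card count and offset from that pile's marker transform, so cards stack.
; Clicks on the stock trigger call OnStockClicked, and the Furr touch area calls OnCardFieldClicked.
; The other four suit touch handlers are empty.
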(event OnClicked(StockTriggerShape)
  (params (TouchedComponent :type Primitive%20Component%20Object%20Reference) (ButtonPressed :type Key%20Structure))
  (Class|MOGTable|OnStockClicked))

(event EventBeginPlay)

(event Collision|EventActorBeginOverlap
  (params (OtherActor :type Actor%20Object%20Reference)))

(event EventTick
  (params (DeltaSeconds :type Float%20%28single-precision%29)))

(event OnClicked(1FurrTouch)
  (params (TouchedComponent :type Primitive%20Component%20Object%20Reference) (ButtonPressed :type Key%20Structure))
  (Class|MOGTable|OnCardFieldClicked 0 false "CS_Furr"))

(event OnClicked(1GemstonesTouch)
  (params (TouchedComponent :type Primitive%20Component%20Object%20Reference) (ButtonPressed :type Key%20Structure)))

(event OnClicked(1BuildingMaterialsTouch)
  (params (TouchedComponent :type Primitive%20Component%20Object%20Reference) (ButtonPressed :type Key%20Structure)))

(event OnClicked(1FoodTouch)
  (params (TouchedComponent :type Primitive%20Component%20Object%20Reference) (ButtonPressed :type Key%20Structure)))

(event OnClicked(1WeaponTouch)
  (params (TouchedComponent :type Primitive%20Component%20Object%20Reference) (ButtonPressed :type Key%20Structure)))

(fn ConstructionScript)

(fn GetStockPlace
  (bind _stockplace (Variables|Default|GetStockPlace))
  (bind _returnvalue (Transformation|GetWorldTransform _stockplace))
  (bind (_location _rotation) (Math|Transform|BreakTransform _returnvalue))
  (bind _asmoggame_mode_base (Utilities|Casting|CastToMOGGameModeBase (Game|GetGameMode))
    (:then
      (bind _returnvalue_2 (Class|MOGGameModeBase|GetNumberOfStockCards _asmoggame_mode_base))
      (return (Math|Transform|MakeTransform (+ (* (Variables|Default|GetCardPlaceOffset) (Math|Conversions|ToInteger(Byte) _returnvalue_2)) _location) _rotation (Variables|Default|GetCardScale))))
    (:CastFailed
      (return ""))))

(fn GetPlayerCardPlace
  (params (PlayerNum :type Byte :default 0) (CardSuit :type ECardSuit%20Enum :default "CS_Weapon"))
  (bind _1weapon (Variables|Default|Get1Weapon))
  (bind _1gemstones (Variables|Default|Get1Gemstones))
  (bind _1furr (Variables|Default|Get1Furr))
  (bind _2weapon (Variables|Default|Get2Weapon))
  (bind _2buidling_materials (Variables|Default|Get2Buidling%20Materials))
  (bind _2food (Variables|Default|Get2Food))
  (bind _2furr (Variables|Default|Get2Furr))
  (bind _2gemstones (Variables|Default|Get2Gemstones))
  (bind _1food (Variables|Default|Get1Food))
  (bind _1building_materials (Variables|Default|Get1Building%20Materials))
  (bind _returnvalue (Utilities|Select :Index CardSuit :CS_Weapon _2weapon :CS_Gemstones _2gemstones :CS_Furr _2furr :CS_Food _2food :CS_Building_Materials _2buidling_materials))
  (bind _returnvalue_2 (Utilities|Select :Index CardSuit :CS_Weapon _1weapon :CS_Gemstones _1gemstones :CS_Furr _1furr :CS_Food _1food :CS_Building_Materials _1building_materials))
  (bind _returnvalue_3 (Transformation|GetWorldTransform _returnvalue))
  (bind _returnvalue_4 (Transformation|GetWorldTransform _returnvalue_2))
  (bind (_location _rotation) (Math|Transform|BreakTransform _returnvalue_3))
  (bind (_location_2 _rotation_2) (Math|Transform|BreakTransform _returnvalue_4))
  (bind _asmoggame_mode_base (Utilities|Casting|CastToMOGGameModeBase (Game|GetGameMode))
    (:then
      (bind _returnvalue_5 (Class|MOGGameModeBase|GetNumberOfPlayerCardsonTable _asmoggame_mode_base PlayerNum CardSuit))
      (if (== PlayerNum 1)
        (return (Math|Transform|MakeTransform (+ _location (* (Variables|Default|GetCardPlaceOffset) (Math|Conversions|ToInteger(Byte) _returnvalue_5))) _rotation (Variables|Default|GetCardScale)))
        (else
          (return (Math|Transform|MakeTransform (+ (* (Variables|Default|GetCardPlaceOffset) (Math|Conversions|ToInteger(Byte) _returnvalue_5)) _location_2) _rotation_2 (Variables|Default|GetCardScale))))))
    (:CastFailed
      (return ""))))

(fn GetNeutralCardPlace
  (params (CardSuit :type ECardSuit%20Enum :default "CS_Weapon"))
  (bind _ngemstones (Variables|Default|GetNGemstones))
  (bind _nfurr (Variables|Default|GetNFurr))
  (bind _nfood (Variables|Default|GetNFood))
  (bind _nbuilding_materials (Variables|Default|GetNBuilding%20Materials))
  (bind _nweapon (Variables|Default|GetNWeapon))
  (bind _returnvalue (Utilities|Select :Index CardSuit :CS_Weapon _nweapon :CS_Gemstones _ngemstones :CS_Furr _nfurr :CS_Food _nfood :CS_Building_Materials _nbuilding_materials))
  (bind _returnvalue_2 (Transformation|GetWorldTransform _returnvalue))
  (bind (_location _rotation) (Math|Transform|BreakTransform _returnvalue_2))
  (bind _asmoggame_mode_base (Utilities|Casting|CastToMOGGameModeBase (Game|GetGameMode))
    (:then
      (bind _returnvalue_3 (Class|MOGGameModeBase|GetNumberOfNeutralCardsonTable _asmoggame_mode_base CardSuit))
      (return (Math|Transform|MakeTransform (+ (* (Variables|Default|GetCardPlaceOffset) (Math|Conversions|ToFloat(Byte) _returnvalue_3)) _location) _rotation (Variables|Default|GetCardScale))))
    (:CastFailed
      (return ""))))